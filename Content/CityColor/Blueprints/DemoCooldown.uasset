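; FairyGUI demo Blueprint that shows looping skill-cooldown indicators built from progress bars.
; On demo start it loads the Cooldown package, creates its Main component at parent size and assigns an icon to each of the two bars.
; Two endlessly repeating linear float tweens of different ranges and durations drive the bar values through update events.
; Demo end removes the package.
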(event `self.OnDemoStart`
  (bind _returnvalue (`GRoot.Get`))
  (`UIPackage.AddPackage` "/Game/CityColor/UI/Cooldown.Cooldown")
  (bind _returnvalue_2 (`UIPackage.CreateObject` "Cooldown" "Main" "/Script/FairyGUI.GComponent"))
  (bind _output_get (set `self.MainView` _returnvalue_2))
  (`GObject.SetParent` _output_get _returnvalue)
  (`GObject.SetSize` _output_get (`GObject.GetSize` _returnvalue) false)
  (`GObject.SetIcon` (`GComponent.GetChild` (`GComponent.GetChild` _output_get "b0" "/Script/FairyGUI.GProgressBar") "icon" null) "/Game/Icons/k0")
  (`GObject.SetIcon` (`GComponent.GetChild` (`GComponent.GetChild` _output_get "b1" "/Script/FairyGUI.GProgressBar") "icon" null) "/Game/Icons/k1")
  (`FairyBlueprintLibrary.TweenFloat` 0.0 100.0 "Linear" 5.0 -1 (delegate `CustomEvent_2`))
  (`FairyBlueprintLibrary.TweenFloat` 10.0 0.0 "Linear" 10.0 -1 (delegate `CustomEvent_3`)))

(event `self.OnDemoEnd`
  (`UIPackage.RemovePackage` "Cooldown"))

(event `CustomEvent_2`
  (params (Value :type "TweenValue Structure (by ref)") (DeltaValue :type "TweenValue Structure (by ref)"))
  (`GProgressBar.SetValue` (`GComponent.GetChild` (stale `self.OnDemoStart` _output_get) "b0" "/Script/FairyGUI.GProgressBar") (`.X` (break `TweenValue` Value))))

(event `CustomEvent_3`
  (params (Value :type "TweenValue Structure (by ref)") (DeltaValue :type "TweenValue Structure (by ref)"))
  (`GProgressBar.SetValue` (`GComponent.GetChild` (stale `self.OnDemoStart` _output_get) "b1" "/Script/FairyGUI.GProgressBar") (`.X` (break `TweenValue` Value))))