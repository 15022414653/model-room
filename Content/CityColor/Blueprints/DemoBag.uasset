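; DemoBag is a FairyGUI bag demo that shows a full-screen main view with a button opening a modal inventory window.
; On start it loads the Bag package and creates the window, with callbacks for content setup and scale-up/scale-down show and hide animations.
; The window's item list is filled with random icons and numbers, and clicking an item copies its icon and text into detail fields.
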(event `self.OnDemoStart`
  (`UIPackage.AddPackage` "/Game/CityColor/UI/Bag.Bag")
  (bind _returnvalue (`UIPackage.CreateObject` "Bag" "Main" "/Script/FairyGUI.GComponent"))
  (bind _output_get (set `self.MainView` _returnvalue))
  (`GObject.SetParent` _output_get (`GRoot.Get`))
  (`GObject.MakeFullScreen` _output_get false)
  (`GComponent.OnClickChild` _output_get "bagBtn" (delegate `OnClickBtn`))
  (bind _returnvalue_2 (`|GenericCreateObject` "/Script/FairyGUI.GWindow" self))
  (bind _output_get_2 (set `self.BagWindow` _returnvalue_2))
  (set `GWindow.InitCallback` (`|CreateDelegate` :!event `InitWindow`) _output_get_2)
  (set `GWindow.ShowingCallback` (delegate `CustomEvent_0`) _output_get_2)
  (set `GWindow.HidingCallback` (delegate `CustomEvent_1`) _output_get_2))

(event `CustomEvent_1`
  (params (Window :type "GWindow Object Reference"))
  (`DemoBlueprintLibrary.ScaleDownWindow` Window))

(event `OnClickBtn`
  (params (EventContext :type "EventContext Object Reference"))
  (`GWindow.Show` (`self.BagWindow`)))

(event `self.OnDemoEnd`
  (`UIPackage.RemovePackage` "Bag"))

(event `CustomEvent_0`
  (params (Window :type "GWindow Object Reference"))
  (`DemoBlueprintLibrary.ScaleUpWindow` Window))

(event `InitWindow`
  (params (Window :type "GWindow Object Reference"))
  (bind _returnvalue (`UIPackage.CreateObject` "Bag" "BagWin" "/Script/FairyGUI.GComponent"))
  (`GWindow.SetContentPane` Window _returnvalue)
  (`GObject.Center` Window false)
  (`GWindow.SetModal` Window true)
  (bind _returnvalue_2 (`GComponent.GetChild` _returnvalue "list" "/Script/FairyGUI.GList"))
  (`GList.SetItemRenderer` _returnvalue_2 (`|CreateDelegate` :!event `ListItemRenderer`))
  (`GList.SetNumItems` _returnvalue_2 45)
  (add `GList.OnClickItem` _returnvalue_2 (`|CreateDelegate` :!event `OnClickItem`)))

(event `ListItemRenderer`
  (params (Index :type Integer) (Obj :type "GObject Object Reference"))
  (bind _returnvalue (`KismetStringLibrary.Conv_IntToString` (`KismetMathLibrary.RandomInteger` 10)))
  (`GObject.SetIcon` Obj (`KismetStringLibrary.Concat_StrStr` "/Game/Icons/i" _returnvalue ".i" _returnvalue))
  (`GObject.SetText` Obj (`KismetStringLibrary.Conv_IntToString` (`KismetMathLibrary.RandomInteger` 100))))

(event `OnClickItem`
  (params (EventContext :type "EventContext Object Reference"))
  (bind _returnvalue (`FairyBlueprintLibrary.GetVariantAsUObject` (`EventContext.GetData` EventContext) "/Script/FairyGUI.GObject"))
  (bind _returnvalue_2 (`GWindow.GetContentPane` (`self.BagWindow`)))
  (`GObject.SetIcon` (`GComponent.GetChild` _returnvalue_2 "n11" null) (`GObject.GetIcon` _returnvalue))
  (`GObject.SetText` (`GComponent.GetChild` _returnvalue_2 "n13" null) (`GObject.GetText` _returnvalue)))