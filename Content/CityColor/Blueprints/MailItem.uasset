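; MailItem is a FairyGUI component Blueprint for a single mail entry in the CityColor UI.
; On construct it caches the time text field, the read and fetched controllers, and a transition.
; Setter functions update the time label and switch each controller between two pages for read and fetched states.
; PlayEffect hides the item, then plays the transition after a caller-supplied delay.
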(event `self.K2_OnConstruct`
  (set `self.TimeText` (`self.GetChild` "timeText" "/Script/FairyGUI.GTextField"))
  (set `self.ReadController` (`self.GetController` "IsRead"))
  (set `self.FetchController` (`self.GetController` "c1"))
  (set `self.Transition` (`self.GetTransition` "t0")))

(fn `PlayEffect`
  (params (Delay :type "Float (double-precision)"))
  (`self.SetVisible` false)
  (`Transition.Play` :`self` (`self.Transition`) :`InDelay` Delay))

(fn `SetFectched`
  (params (Fetched :type Boolean))
  (bind _fetchcontroller (`self.FetchController`))
  (if Fetched
    (`GController.SetSelectedIndex` _fetchcontroller 1)
    (else
      (`GController.SetSelectedIndex` _fetchcontroller 0))))

(fn `SetRead`
  (params (Read :type Boolean))
  (bind _readcontroller (`self.ReadController`))
  (if Read
    (`GController.SetSelectedIndex` _readcontroller 1)
    (else
      (`GController.SetSelectedIndex` _readcontroller 0))))

(fn `SetTime`
  (params (Time :type String))
  (`self.SetText` (`self.TimeText`) Time))