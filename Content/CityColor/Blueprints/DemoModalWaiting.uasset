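; FairyGUI demo Blueprint showing global and per-window modal waiting overlays.
; On start it sets both overlay resources in the UI config, loads the ModalWaiting package, and builds the main view and a test window.
; A global wait shows immediately; one button opens the centered window, whose own button triggers a window-level wait.
; Timers close each overlay after a short delay, and demo end removes the package.
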(event `self.OnDemoStart`
  (bind _structout (setmembers `UIConfig` :`StructRef` (`FairyBlueprintLibrary.GetUIConfig`) :`GlobalModalWaiting` "ui://ModalWaiting/GlobalModalWaiting" :`WindowModalWaiting` "ui://ModalWaiting/WindowModalWaiting"))
  (`FairyBlueprintLibrary.SetUIConfig` _structout)
  (`UIPackage.AddPackage` "/Game/CityColor/UI/ModalWaiting.ModalWaiting")
  (bind _returnvalue (`UIPackage.CreateObject` "ModalWaiting" "Main" "/Script/FairyGUI.GComponent"))
  (bind _output_get (set `self.MainView` _returnvalue))
  (`GObject.SetParent` _output_get (`GRoot.Get`))
  (`GObject.MakeFullScreen` _output_get false)
  (`GComponent.OnClickChild` _output_get "n0" (delegate `CustomEvent_2`))
  (bind _returnvalue_2 (`GWindow.CreateWindow` "ModalWaiting" "TestWin"))
  (bind _output_get_2 (set `self.TestWin` _returnvalue_2))
  (`GComponent.OnClickChild` (`GWindow.GetContentPane` _output_get_2) "n1" (delegate `CustomEvent_0`))
  (`GRoot.ShowModalWait` (`GRoot.Get`))
  (`KismetSystemLibrary.K2_SetTimerDelegate` (delegate `CustomEvent_3`) 3.0))

(event `CustomEvent_2`
  (params (EventContext :type "EventContext Object Reference"))
  (bind _testwin (`self.TestWin`))
  (`GWindow.Show` _testwin)
  (`GObject.Center` _testwin false))

(event `CustomEvent_0`
  (params (EventContext :type "EventContext Object Reference"))
  (`GWindow.ShowModalWait` (stale `self.OnDemoStart` _output_get_2) 0)
  (`KismetSystemLibrary.K2_SetTimerDelegate` (delegate `CustomEvent_1`) 3.0))

(event `CustomEvent_3`
  (`GRoot.CloseModalWait` (`GRoot.Get`)))

(event `self.OnDemoEnd`
  (`UIPackage.RemovePackage` "ModalWaiting"))

(event `CustomEvent_1`
  (`GWindow.CloseModalWait` (stale `self.OnDemoStart` _output_get_2) 0))