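; FairyGUI demo Blueprint that showcases UI transition animations, each launched from a button on a fullscreen main view.
; It pre-creates six components from the Transition package; a clicked button hides the button group, adds its component and plays transition "t0".
; Completion removes the component and restores the buttons.
; The PowerUp effect also randomizes a gain and uses a transition label hook to start a tweened number count-up.
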(event `self.OnDemoStart`
  (bind _mainview (`self.MainView`))
  (`UIPackage.AddPackage` "/Game/CityColor/UI/Transition.Transition")
  (bind _returnvalue (`UIPackage.CreateObject` "Transition" "Main" "/Script/FairyGUI.GComponent"))
  (bind _output_get (set `self.MainView` _returnvalue))
  (`GObject.MakeFullScreen` _output_get false)
  (bind _returnvalue_2 (`UIPackage.CreateObject` "Transition" "BOSS" "/Script/FairyGUI.GComponent"))
  (set `self.g0` _returnvalue_2)
  (bind _returnvalue_3 (`UIPackage.CreateObject` "Transition" "BOSS_SKILL" "/Script/FairyGUI.GComponent"))
  (set `self.g1` _returnvalue_3)
  (bind _returnvalue_4 (`UIPackage.CreateObject` "Transition" "TRAP" "/Script/FairyGUI.GComponent"))
  (set `self.g2` _returnvalue_4)
  (bind _returnvalue_5 (`UIPackage.CreateObject` "Transition" "GoodHit" "/Script/FairyGUI.GComponent"))
  (bind _output_get_2 (set `self.g3` _returnvalue_5))
  (`GObject.SetPosition` _output_get_2 (`KismetMathLibrary.MakeVector2D` (- (`GObject.GetWidth` (`self.MainView`)) 270.0) 100.0))
  (bind _returnvalue_6 (`UIPackage.CreateObject` "Transition" "PowerUp" "/Script/FairyGUI.GComponent"))
  (set `self.g4` _returnvalue_6)
  (bind _returnvalue_7 (`UIPackage.CreateObject` "Transition" "PathDemo" "/Script/FairyGUI.GComponent"))
  (set `self.g5` _returnvalue_7)
  (`GComponent.AddChild` (`GRoot.Get`) _mainview)
  (set `self.Btns` (`GComponent.GetChild` _mainview "g0" null))
  (`GComponent.OnClickChild` _mainview "btn0" (delegate `CustomEvent_6`))
  (`GComponent.OnClickChild` _mainview "btn1" (delegate `CustomEvent_7`))
  (`GComponent.OnClickChild` _mainview "btn2" (delegate `CustomEvent_8`))
  (`GComponent.OnClickChild` _mainview "btn3" (delegate `CustomEvent_9`))
  (`GComponent.OnClickChild` _mainview "btn4" (delegate `CustomEvent_10`))
  (`GComponent.OnClickChild` _mainview "btn5" (delegate `CustomEvent_11`)))

(event `self.OnDemoEnd`
  (`UIPackage.RemovePackage` "Transition"))

(event `CustomEvent_6`
  (params (EventContext :type "EventContext Object Reference"))
  (`self.PlayTransition` (`self.g0`) 1))

(event `CustomEvent_7`
  (params (EventContext :type "EventContext Object Reference"))
  (`self.PlayTransition` (`self.g1`) 1))

(event `CustomEvent_8`
  (params (EventContext :type "EventContext Object Reference"))
  (`self.PlayTransition` (`self.g2`) 1))

(event `CustomEvent_9`
  (params (EventContext :type "EventContext Object Reference"))
  (`self.PlayTransition` (`self.g3`) 3))

(event `CustomEvent_10`
  (params (EventContext :type "EventContext Object Reference"))
  (`self.PlayTransition2`))

(event `CustomEvent_11`
  (params (EventContext :type "EventContext Object Reference"))
  (`self.PlayTransition` (`self.g5`)))

(event `PlayComplete`
  (`GComponent.RemoveChildAt` (`GRoot.Get`) 1)
  (`GObject.SetVisible` (`self.Btns`) true))

(fn `PlayNumberHook`
  (`FairyBlueprintLibrary.TweenFloat` (`self.StartValue`) (`self.EndValue`) "Linear" 0.3 0 (`|CreateDelegate` :!event `PlayNumberUpdate`)))

(fn `PlayNumberUpdate`
  (params (Value :type "TweenValue Structure (by ref)") (DeltaValue :type "TweenValue Structure (by ref)"))
  (`GObject.SetText` (`GComponent.GetChild` (`self.g4`) "value" null) (`KismetStringLibrary.Conv_IntToString` (`KismetMathLibrary.FFloor` (`.X` (break `TweenValue` Value))))))

(fn `PlayTransition`
  (params (Target :type "GComponent Object Reference") (Times :type Integer))
  (`GComponent.AddChild` (`GRoot.Get`) Target)
  (`GObject.SetVisible` (`self.Btns`) false)
  (`Transition.Play` (`GComponent.GetTransition` Target "t0") (`|CreateDelegate` :!event `PlayComplete`) Times 0.0 0.0 -1.0))

(fn `PlayTransition2`
  (bind _g4 (`self.g4`))
  (bind _g4_2 (`self.g4`))
  (bind _returnvalue (`GComponent.GetTransition` _g4 "t0"))
  (bind _returnvalue_2 (`KismetMathLibrary.FFloor` (* (`KismetMathLibrary.RandomFloatInRange` 0.0 1.0) 2000.0)))
  (`GComponent.AddChild` (`GRoot.Get`) _g4)
  (`GObject.SetPosition` _g4 (`KismetMathLibrary.MakeVector2D` 20.0 (- (`GObject.GetHeight` (`self.MainView`)) 220.0)))
  (bind _output_get (set `self.StartValue` 10000.0))
  (set `self.EndValue` (+ _output_get (`KismetMathLibrary.Conv_IntToDouble` _returnvalue_2)))
  (`GObject.SetText` (`GComponent.GetChild` _g4_2 "value" null) (`KismetStringLibrary.Conv_DoubleToString` _output_get))
  (`GObject.SetText` (`GComponent.GetChild` _g4_2 "add_value" null) (`KismetStringLibrary.Concat_StrStr` "+" (`KismetStringLibrary.Conv_IntToString` _returnvalue_2)))
  (`GObject.SetVisible` (`self.Btns`) false)
  (`Transition.SetHook` _returnvalue "play_num_now" (`|CreateDelegate` :!event `PlayNumberHook`))
  (`Transition.Play` _returnvalue (`|CreateDelegate` :!event `PlayComplete`) 1 0.0 0.0 -1.0))