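; FairyGUI demo of nested scrolling: a virtual list of 1000 items, each with its own scroll pane and Stick and Delete buttons.
; The item renderer labels each row, resets its scroll position and binds both buttons to report the clicked row in a text field.
; Touching the list snaps scrolled rows closed and cancels dragging, unless the touch is on that row's buttons.
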(event `self.OnDemoStart`
  (`UIPackage.AddPackage` "/Game/CityColor/UI/ScrollPane.ScrollPane")
  (bind _returnvalue (`UIPackage.CreateObject` "ScrollPane" "Main" "/Script/FairyGUI.GComponent"))
  (bind _output_get (set `self.MainView` _returnvalue))
  (`GObject.SetParent` _output_get (`GRoot.Get`))
  (`GObject.MakeFullScreen` _output_get false)
  (bind _output_get_2 (set `self.List` (`GComponent.GetChild` _output_get "list" "/Script/FairyGUI.GList")))
  (`GList.SetItemRenderer` _output_get_2 (`|CreateDelegate` :!event `ListItemRenderer`))
  (`GList.SetVirtual` _output_get_2)
  (`GList.SetNumItems` _output_get_2 1000)
  (add `GObject.OnTouchBegin` _output_get_2 (`|CreateDelegate` :!event `OnListTouchBegin`)))

(event `self.OnDemoEnd`
  (`UIPackage.RemovePackage` "ScrollPane"))

(event `ListItemRenderer`
  (params (Index :type Integer) (Obj :type "GObject Object Reference"))
  (`GObject.SetText` Obj (`KismetStringLibrary.Conv_IntToString` Index))
  (bind _asgcomponent (cast `GComponent` Obj))
  (`ScrollPane.SetPosX` (`GComponent.GetScrollPane` _asgcomponent) 0.0 false)
  (`GComponent.OnClickChild` _asgcomponent "b0" (`|CreateDelegate` :!event `OnClickStick`))
  (`GComponent.OnClickChild` _asgcomponent "b1" (`|CreateDelegate` :!event `OnClickDelete`)))

(event `OnListTouchBegin`
  (params (EventContext :type "EventContext Object Reference"))
  (bind _returnvalue (`EventContext.GetInitiator` EventContext))
  (for _index (range (`GComponent.NumChildren` (`self.List`)))
    (bind _returnvalue_2 (`GComponent.GetChildAt` (`self.List`) _index "/Script/FairyGUI.GComponent"))
    (bind _returnvalue_3 (`GComponent.GetScrollPane` _returnvalue_2))
    (if (!= (`ScrollPane.GetPosX` _returnvalue_3) 0.0)
      (if (not (or (`GComponent.IsAncestorOf` (`GComponent.GetChild` _returnvalue_2 "b0" "/Script/FairyGUI.GComponent") _returnvalue) (`GComponent.IsAncestorOf` (`GComponent.GetChild` _returnvalue_2 "b1" "/Script/FairyGUI.GComponent") _returnvalue)))
        (`ScrollPane.SetPosX` _returnvalue_3 0.0 true)
        (`ScrollPane.CancelDragging` _returnvalue_3)
        (`ScrollPane.CancelDragging` (`GComponent.GetScrollPane` (`self.List`)))))))

(event `OnClickStick`
  (params (EventContext :type "EventContext Object Reference"))
  (`GObject.SetText` (`GComponent.GetChild` (`self.MainView`) "txt" null) (`KismetStringLibrary.Concat_StrStr` "Stick " (`GObject.GetText` (`GObject.GetParent` (`EventContext.GetSender` EventContext))))))

(event `OnClickDelete`
  (params (EventContext :type "EventContext Object Reference"))
  (`GObject.SetText` (`GComponent.GetChild` (`self.MainView`) "txt" null) (`KismetStringLibrary.Concat_StrStr` "Delete " (`GObject.GetText` (`GObject.GetParent` (`EventContext.GetSender` EventContext))))))