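; FairyGUI demo Blueprint for a virtual looping list with a center-zoom carousel effect.
; On start it loads the LoopList package, creates the full-screen Main view and fills the list with numbered icons pivoted at their centers.
; Each scroll enlarges items by their distance from the view's middle and writes the middle item's index to a text child.
; The package is removed when the demo ends.
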(event `self.OnDemoStart`
  (`UIPackage.AddPackage` "/Game/CityColor/UI/LoopList.LoopList")
  (bind _returnvalue (`UIPackage.CreateObject` "LoopList" "Main" "/Script/FairyGUI.GComponent"))
  (bind _output_get (set `self.MainView` _returnvalue))
  (`GObject.SetParent` _output_get (`GRoot.Get`))
  (`GObject.MakeFullScreen` _output_get false)
  (bind _output_get_2 (set `self.List` (`GComponent.GetChild` _output_get "list" "/Script/FairyGUI.GList")))
  (`GList.SetItemRenderer` _output_get_2 (`|CreateDelegate` :!event `ListItemRenderer`))
  (`GList.SetVirtualAndLoop` _output_get_2)
  (add `GComponent.OnScroll` _output_get_2 (`|CreateDelegate` :!event `HandleScroll`))
  (`GList.SetNumItems` _output_get_2 5)
  (`self.HandleScroll` null))

(event `self.OnDemoEnd`
  (`UIPackage.RemovePackage` "LoopList"))

(event `ListItemRenderer`
  (params (Index :type Integer) (Obj :type "GObject Object Reference"))
  (`GObject.SetPivot` Obj (`KismetMathLibrary.MakeVector2D` 0.5 0.5) false)
  (`GObject.SetIcon` Obj (`KismetStringLibrary.Concat_StrStr` "ui://LoopList/n" (`KismetStringLibrary.Conv_IntToString` (+ Index 1)))))

(fn `HandleScroll`
  (params (EventContext :type "EventContext Object Reference"))
  (locals (MidX :type "Float (double-precision)") (Obj :type "GObject Object Reference") (Dist :type "Float (double-precision)"))
  (bind _list (`self.List`))
  (bind _obj (`local.Obj`))
  (bind _list_2 (`self.List`))
  (bind _list_3 (`self.List`))
  (bind _obj_2 (`local.Obj`))
  (bind _returnvalue (+ 1.0 (* (- 1.0 (/ (`local.Dist`) (`GObject.GetWidth` (`local.Obj`)))) 0.24)))
  (set `local.MidX` (+ (`ScrollPane.GetPosX` (`GComponent.GetScrollPane` _list)) (* (`GComponent.GetViewWidth` _list) 0.5)))
  (for _index (range (`GComponent.NumChildren` _list_3))
    (set `local.Obj` (`GComponent.GetChildAt` _list_3 _index null))
    (set `local.Dist` (`KismetMathLibrary.Abs` (- (- (`local.MidX`) (`GObject.GetX` _obj)) (* (`GObject.GetWidth` _obj) 0.5))))
    (if (> (`local.Dist`) (`GObject.GetWidth` (`local.Obj`)))
      (`GObject.SetScale` _obj_2 (`KismetMathLibrary.Vector2D_One`))
      (else
        (`GObject.SetScale` _obj_2 (`KismetMathLibrary.MakeVector2D` _returnvalue _returnvalue)))))
  (`GObject.SetText` (`GComponent.GetChild` (`self.MainView`) "n3" null) (`KismetStringLibrary.Conv_IntToString` (mod (+ (`GComponent.GetFirstChildInView` _list_2) 1) (`GList.GetNumItems` _list_2)))))