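; DemoGuide is a FairyGUI demo of a tutorial guide overlay that highlights the bag button.
; On start it loads the Guide package, builds the main view and prepares a full-screen GuideLayer.
; A child click attaches the layer to root, then after a short timer maps the button's rect into layer space, resizing and tweening the window onto it.
; Clicking the bag button removes the layer; demo end removes the package.
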(event `OnClick_Event_0`
  (params (EventContext :type "EventContext Object Reference"))
  (`GObject.RemoveFromParent` (`self.GuideLayer`)))

(event `self.OnDemoStart`
  (bind _returnvalue (`GRoot.Get`))
  (`UIPackage.AddPackage` "/Game/CityColor/UI/Guide.Guide")
  (bind _returnvalue_2 (`UIPackage.CreateObject` "Guide" "Main" "/Script/FairyGUI.GComponent"))
  (bind _output_get (set `self.MainView` _returnvalue_2))
  (`GObject.SetParent` _output_get _returnvalue)
  (`GObject.SetSize` _output_get (`GObject.GetSize` _returnvalue) false)
  (set `self.BagButton` (`GComponent.GetChild` _output_get "bagBtn" null))
  (bind _returnvalue_3 (`UIPackage.CreateObject` "Guide" "GuideLayer" "/Script/FairyGUI.GComponent"))
  (bind _output_get_2 (set `self.GuideLayer` _returnvalue_3))
  (`GObject.MakeFullScreen` _output_get_2 true)
  (`GComponent.OnClickChild` (`self.MainView`) "n2" (delegate `OnClickShowGuide`))
  (add `GObject.OnClick` (`self.BagButton`) (delegate `OnClick_Event_0`)))

(event `OnClickShowGuide`
  (params (EventContext :type "EventContext Object Reference"))
  (`GObject.SetParentToRoot` (`self.GuideLayer`))
  (`KismetSystemLibrary.K2_SetTimerDelegate` (delegate `CustomEvent_0`) 0.1))

(event `self.OnDemoEnd`
  (`UIPackage.RemovePackage` "Guide"))

(event `CustomEvent_0`
  (bind _bagbutton (`self.BagButton`))
  (bind _guidelayer (`self.GuideLayer`))
  (bind _returnvalue (`GComponent.GetChild` _guidelayer "window" null))
  (bind _returnvalue_2 (`GObject.LocalToGlobalRect` _bagbutton (`KismetMathLibrary.MakeBox2D` (0.0 0.0) (`GObject.GetSize` _bagbutton))))
  (bind _returnvalue_3 (`GObject.GlobalToLocalRect` _guidelayer _returnvalue_2))
  (bind (_min _max) (break `Box2D` _returnvalue_3))
  (`GObject.SetSize` _returnvalue (- _max _min) false)
  (`FairyBlueprintLibrary.TweenVector2` (`GObject.GetPosition` _returnvalue) _min "CubicOut" 0.5 0 (delegate `CustomEvent_2`)))

(event `CustomEvent_2`
  (params (Value :type "TweenValue Structure (by ref)") (DeltaValue :type "TweenValue Structure (by ref)"))
  (bind (_x _y) (break `TweenValue` Value))
  (`GObject.SetPosition` (`GComponent.GetChild` (`self.GuideLayer`) "window" null) (`KismetMathLibrary.MakeVector2D` _x _y)))